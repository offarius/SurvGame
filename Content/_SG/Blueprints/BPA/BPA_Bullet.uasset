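; BPA_Bullet is a reusable projectile with a Paper2D flipbook visual, apparently built for pooling.
; SetupBulletProperties configures look, scale, velocity, damage, target tag and causer, enables Pawn overlap and starts a lifespan timer.
; On expiry, ResetStatusByTimer clears visual, motion, collision and hit list, then parks the actor off-level instead of destroying it.
; Sphere overlaps record each tagged target once, but only print its name; damage is never applied.
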(event `self.Sphere.OnComponentBeginOverlap`
  (params (OverlappedComponent :type "PrimitiveComponent Object Reference") (OtherActor :type "Actor Object Reference") (OtherComp :type "PrimitiveComponent Object Reference") (OtherBodyIndex :type Integer) (bFromSweep :type Boolean) (SweepResult :type "HitResult Structure (by ref)"))
  (bind _ref_player (`/Game/_SG/Data/GI_SG.Ref_Player` (`/Game/_SG/Data/Flib_GI.Flib_GetGI`)))
  (`/Engine/EditorBlueprintResources/StandardMacros.IsValid` OtherActor
    (:`Is Valid`
      (if (and (`self.ActorHasTag` OtherActor (`self.AppliedTargetTag`)) (not (`KismetArrayLibrary.Array_Contains` (`self.DamagedActorList`) OtherActor)))
        (bind _output_get (set `self.HitTarget` OtherActor))
        (`KismetArrayLibrary.Array_AddUnique` (`self.DamagedActorList`) _output_get)
        (if (and (`KismetSystemLibrary.IsValid` _ref_player) (not (`/Game/_SG/Blueprints/BP_Player.Dead` _ref_player)))
          (`KismetSystemLibrary.PrintString` (`KismetSystemLibrary.GetDisplayName` (`self.HitTarget`))))))))

(fn `ResetStatusByTimer`
  (`PaperFlipbookComponent.SetFlipbook` (`self.PaperFlipbook`) null)
  (`KismetArrayLibrary.Array_Clear` (`self.DamagedActorList`))
  (set `MovementComponent.Velocity` (0.0 0.0 0.0) (`self.ProjectileMovement`))
  (`SceneComponent.SetWorldScale3D` (`self.Capsule`) (1.0 1.0 1.0))
  (`SceneComponent.SetWorldScale3D` (`self.Sphere`) (1.0 1.0 1.0))
  (`SceneComponent.SetWorldScale3D` (`self.PaperFlipbook`) (1.0 1.0 1.0))
  (`PrimitiveComponent.SetCollisionResponseToAllChannels` (`self.Sphere`) "ECR_Ignore")
  (`PrimitiveComponent.SetCollisionResponseToAllChannels` (`self.Capsule`) "ECR_Ignore")
  (`self.K2_SetActorLocation` (0.0 1000.0 -10000.0))
  (set `self.BulletState` "NewEnumerator1"))

(fn `SetupBulletProperties`
  (params (OverallScale :type "Vector Structure") (Damage :type "Float (double-precision)") (ProjectileVel :type "Vector Structure") (TargetTag :type Name) (DamageCauser :type "Actor Object Reference") (NewFlipbook :type "PaperFlipbook Object Reference") (FlipbookScale :type "Vector Structure") (SpecifiedLifeSpan :type "Float (double-precision)"))
  (`PaperFlipbookComponent.SetFlipbook` (`self.PaperFlipbook`) (`local.NewFlipbook`))
  (`SceneComponent.SetWorldScale3D` (`self.Sphere`) (`local.OverallScale`))
  (`SceneComponent.SetWorldScale3D` (`self.PaperFlipbook`) (`local.FlipbookScale`))
  (set `MovementComponent.Velocity` (`local.ProjectileVel`) (`self.ProjectileMovement`))
  (set `self.AppliedDamage` (`local.Damage`))
  (set `self.AppliedTargetTag` (`local.TargetTag`))
  (set `self.AppliedDamageCauser` (`local.DamageCauser`))
  (set `self.BulletState` "NewEnumerator0")
  (`PrimitiveComponent.SetCollisionResponseToChannel` (`self.Sphere`) "ECC_Pawn" "ECR_Overlap")
  (`PrimitiveComponent.SetCollisionResponseToChannel` (`self.Capsule`) "ECC_Pawn" "ECR_Overlap")
  (`KismetSystemLibrary.K2_SetTimer` null "ResetStatusByTimer" (`local.SpecifiedLifeSpan`)))

(fn `UserConstructionScript`)