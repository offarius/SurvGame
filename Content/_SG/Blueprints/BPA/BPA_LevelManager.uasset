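; Level manager actor that registers itself with the game instance on BeginPlay and serves as the bullet object pool for the level.
; PoolingBullets reuses the first available bullet in the pool, or spawns a new BPA_Bullet at a remote location and adds it, so the pool grows on demand.
; It then configures that bullet's damage, velocity, target tag, flipbook visuals and lifespan before moving it to the requested location.
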(event `self.ReceiveBeginPlay`
  (set `/Game/_SG/Data/GI_SG.Ref_LevelManager` self (`/Game/_SG/Data/Flib_GI.Flib_GetGI`)))

(event `self.ReceiveTick`
  (params (DeltaSeconds :type "Float (single-precision)"))
  ;[1 1 1] Test
)

(fn `PoolingBullets`
  (params (Location :type "Vector Structure") (OverallScale :type "Vector Structure") (Damage :type "Float (double-precision)") (ProjectileVel :type "Vector Structure") (TargetTag :type Name) (DamageCauser :type "Actor Object Reference") (NewFlipbook :type "PaperFlipbook Object Reference") (FlipbookScale :type "Vector Structure") (LifeSpan :type "Float (double-precision)"))
  (locals (L_AvailableBullet :type "/Game/_SG/Blueprints/BPA/BPA_Bullet Object Reference"))
  (bind _l_availablebullet (`local.L_AvailableBullet`))
  (for _array_element (`self.BulletPool`)
    (if (`|EnumEquality` (`/Game/_SG/Blueprints/BPA/BPA_Bullet.BulletState` _array_element) "NewEnumerator1")
      (set `local.L_AvailableBullet` _array_element)
      (break)))
  (`local.L_AvailableBullet`
    (:`then`
      _)
    (:`else`
      (bind _returnvalue (`|SpawnActorFromClass` "/Game/_SG/Blueprints/BPA/BPA_Bullet.BPA_Bullet_C" (`KismetMathLibrary.MakeTransform` (0.0 1000.0 -10000.0)) "AdjustIfPossibleButAlwaysSpawn" "MultiplyWithRoot" null "None" null))
      (bind _output_get (set `local.L_AvailableBullet` _returnvalue))
      (`KismetArrayLibrary.Array_Add` (`self.BulletPool`) _output_get)))
  (`/Game/_SG/Blueprints/BPA/BPA_Bullet.SetupBulletProperties` _l_availablebullet (`local.OverallScale`) (`local.Damage`) (`local.ProjectileVel`) (`local.TargetTag`) (`local.DamageCauser`) (`local.NewFlipbook`) (`local.FlipbookScale`) LifeSpan)
  (`self.K2_SetActorLocation` _l_availablebullet (`local.Location`) false false))

(fn `UserConstructionScript`)